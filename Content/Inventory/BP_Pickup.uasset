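; World pickup actor for inventory items, showing a mesh and an optional floating name widget, that destroys itself when interacted with.
; Its construction script, on the server only, looks up ItemRowName in a data table to set name, mesh, scale, offset and name display.
; BeginPlay passes the name to the widget, and SetItemnameVisibility toggles it only when name display is enabled.
; The interact hint is empty and no inventory transfer happens here.
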(event EventBeginPlay
  (bind _aswb_pickup_item_name (Utilities|Casting|CastToWB_PickupItemName (UserInterface|GetUserWidgetObject (Variables|Default|GetWidget_PickupName))))
  (Default|SetTextItemName _aswb_pickup_item_name (Variables|Default|GetPickup%20Name)))

(event EventInteractwithActor
  (params (PlayerCharacter :type Third%20Person%20Character%20Object%20Reference))
  (Actor|DestroyActor))

(event EventSetItemnameVisibility
  (params (NewVisibility :type Boolean))
  (if (Variables|Default|GetShow%20Pickup%20Name)
    (Rendering|SetVisibility (Variables|Default|GetWidget_PickupName) NewVisibility false)))

(fn ConstructionScript
  (bind _pickupmesh (Variables|Default|GetPickupMesh))
  (if (Networking|IsServer)
    (bind _returnvalue (Utilities|GetDataTableRow "/Game/Inventory/PickupItemInfo_Table.PickupItemInfo_Table" (Variables|Default|GetItemRowName))
      (:then
        (Variables|Default|SetPickup%20Name (.PickupName (Utilities|Struct|BreakS_PickupItemInfo _returnvalue)))
        (Components|StaticMesh|SetStaticMesh _pickupmesh (.PickupMesh (Utilities|Struct|BreakS_PickupItemInfo _returnvalue)))
        (Transformation|SetRelativeScale3D _pickupmesh (Math|Vector|MakeVector (.PickupMesh_Scale (Utilities|Struct|BreakS_PickupItemInfo _returnvalue)) (.PickupMesh_Scale (Utilities|Struct|BreakS_PickupItemInfo _returnvalue)) (.PickupMesh_Scale (Utilities|Struct|BreakS_PickupItemInfo _returnvalue))))
        (Variables|Default|SetShow%20Pickup%20Name (.ShowPickupName (Utilities|Struct|BreakS_PickupItemInfo _returnvalue)))
        (Transformation|SetRelativeLocation _pickupmesh (.PickupMeshOffset (Utilities|Struct|BreakS_PickupItemInfo _returnvalue)) false false)))))

(fn GetInteractHintText
  (return ""))